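; SoS_Beacon is a destructible, spinning beacon actor whose destruction counts as the player's death in Tower Panic.
; On BeginPlay it randomizes its RotatingMovement rate on all three axes and binds its damage and death events.
; Any damage taken is forwarded to BeaconHealthSystem.
; When that component reports death, the beacon calls CustomEventPlayerDied on TowerPanic_GameState and destroys itself.
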(event `self.ReceiveBeginPlay`
  (add `self.OnTakeAnyDamage` (delegate `OnTakeAnyDamage_Event`))
  (`self.RandomizeRotation`)
  (add `/Game/MyContent/Blueprints/HealthSystem.OnIsDead` (`self.BeaconHealthSystem`) (delegate `CustomEvent_OnIsDead`)))

(event `OnTakeAnyDamage_Event` :!signature `self.OnTakeAnyDamage`
  (params (DamagedActor :type "Actor Object Reference") (Damage :type "Float (single-precision)") (DamageType :type "DamageType Object Reference") (InstigatedBy :type "Controller Object Reference") (DamageCauser :type "Actor Object Reference"))
  (`/Game/MyContent/Blueprints/HealthSystem.Damage` (`self.BeaconHealthSystem`) Damage null))

(event `CustomEvent_OnIsDead`
  (`/Game/MyContent/Blueprints/TowerPanic_GameState.CustomEvent_PlayerDied` (cast `/Game/MyContent/Blueprints/TowerPanic_GameState` (`GameplayStatics.GetGameState`) :!pure true))
  (`self.K2_DestroyActor`))

(fn `RandomizeRotation`
  (set `RotatingMovementComponent.RotationRate` (`KismetMathLibrary.MakeRotator` (`KismetMathLibrary.RandomFloatInRange` 0.0 180.0) (`KismetMathLibrary.RandomFloatInRange` 0.0 180.0) (`KismetMathLibrary.RandomFloatInRange` 0.0 180.0)) (`self.RotatingMovement`)))

(fn `UserConstructionScript`)