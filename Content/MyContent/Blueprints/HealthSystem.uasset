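; Reusable health system Blueprint that tracks current health and signals health changes and death.
; On BeginPlay it adds StartingHealth through UpdateHealth, which Heal and Damage also use, with Damage negating its amount.
; UpdateHealth broadcasts OnHealthUpdate, then OnIsDead when health is zero or below, without clamping.
; ResetHealth sets health directly to MaxHealth without broadcasting.
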(event `self.ReceiveBeginPlay`
  (`self.UpdateHealth` (`self.StartingHealth`)))

(fn `Damage`
  (params (`Damage Amount` :type "Float (double-precision)"))
  (`self.UpdateHealth` (* `Damage Amount` -1.0)))

(fn `Heal`
  (params (AmountHealed :type "Float (double-precision)"))
  (`self.UpdateHealth` AmountHealed))

(fn `ResetHealth`
  (set `self.CurrentHealth` (`self.MaxHealth`)))

(fn `UpdateHealth`
  (params (HealthChange :type "Float (double-precision)"))
  (bind _output_get (set `self.CurrentHealth` (+ HealthChange (`self.CurrentHealth`))))
  (`self.OnHealthUpdate` _output_get)
  (if (<= _output_get 0.0)
    (`self.OnIsDead`)))