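; Player character Blueprint for TowerPanic that connects incoming damage and death to the player state and animation.
; On BeginPlay it caches the ABP_Player anim instance and binds to its own damage event and the TowerPanic_PlayerState IsDead dispatcher.
; Damage is forwarded to the player state, which signals death back.
; On death the character flags itself dead, calls TryToKill on the anim instance and disables movement.
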(event `self.ReceiveBeginPlay`
  (add `self.OnTakeAnyDamage` (delegate `OnTakeAnyDamage_Event`))
  (bind _asabp_player (cast `/Game/MyContent/Characters/Player/Animations/ABP_Player` (`SkeletalMeshComponent.GetAnimInstance` (`self.Mesh`))))
  (set `self.ABP Player` _asabp_player)
  (add `/Game/MyContent/Blueprints/TowerPanic_PlayerState.IsDead` (cast `/Game/MyContent/Blueprints/TowerPanic_PlayerState` (`self.PlayerState`) :!pure true) (delegate `PlayerIsDead`)))

(event `OnTakeAnyDamage_Event` :!signature `self.OnTakeAnyDamage`
  (params (DamagedActor :type "Actor Object Reference") (Damage :type "Float (single-precision)") (DamageType :type "DamageType Object Reference") (InstigatedBy :type "Controller Object Reference") (DamageCauser :type "Actor Object Reference"))
  (`/Game/MyContent/Blueprints/TowerPanic_PlayerState.Damage` (cast `/Game/MyContent/Blueprints/TowerPanic_PlayerState` (`self.PlayerState`) :!pure true) Damage))

(event `PlayerIsDead`
  (params (IsDead :type Boolean))
  (set `self.IsDead` true)
  (`/Game/MyContent/Characters/Player/Animations/ABP_Player.TryToKill` (`self.ABP Player`))
  (`CharacterMovementComponent.DisableMovement` (`self.CharacterMovement`)))

(fn `UserConstructionScript`)