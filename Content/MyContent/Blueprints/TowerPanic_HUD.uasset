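; TowerPanic HUD that switches the on-screen widget between the game, death and win screens.
; On BeginPlay it shows the game UI and binds to the game state's player-died and player-won events, each handled once through its own DoOnce.
; UpdateUI removes the current widget, then creates the requested class for the owning player and adds it to the viewport.
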(event `self.ReceiveBeginPlay`
  ;[1 1 1] Setup
  (`self.UpdateUI` "/Game/MyContent/UI/TowerPanic_GameUI.TowerPanic_GameUI_C")
  (add `/Game/MyContent/Blueprints/TowerPanic_GameState.OnPlayerDied` (cast `/Game/MyContent/Blueprints/TowerPanic_GameState` (`GameplayStatics.GetGameState`) :!pure true) (delegate `CustomEvent_OnPlayerLost`))
  (add `/Game/MyContent/Blueprints/TowerPanic_GameState.OnPlayerWon` (cast `/Game/MyContent/Blueprints/TowerPanic_GameState` (`GameplayStatics.GetGameState`) :!pure true) (delegate `CustomEvent_PlayerWon`)))

(event `CustomEvent_OnPlayerLost`
  ;[1 1 1] Sets UI to DeathUI
  (`/Engine/EditorBlueprintResources/StandardMacros.DoOnce` false
    (:`Completed`
      (`self.UpdateUI` "/Game/MyContent/UI/DeathUI.DeathUI_C"))))

(event `CustomEvent_PlayerWon`
  ;[1 1 1] Sets UI to WinUI
  (`/Engine/EditorBlueprintResources/StandardMacros.DoOnce` false
    (:`Completed`
      (`self.UpdateUI` "/Game/MyContent/UI/WinUI.WinUI_C"))))

(fn `UpdateUI`
  (params (Class :type "UserWidget Class Reference"))
  (bind _current_ui (`self.Current UI`))
  (`|ExecutionSequence`
    (:`then_0`
      ;[1 1 1] If UI already exists we remove it
      (`/Engine/EditorBlueprintResources/StandardMacros.IsValid` _current_ui
        (:`Is Valid`
          (`Widget.RemoveFromParent` _current_ui))))
    (:`then_1`
      ;[1 1 1] Creates and adds new UI Widget
      (bind _returnvalue (`|CreateWidget` Class (`self.PlayerOwner`)))
      (bind _output_get (set `self.Current UI` _returnvalue))
      (`UserWidget.AddToViewport` _output_get 0)
      (return))))

(fn `UserConstructionScript`)