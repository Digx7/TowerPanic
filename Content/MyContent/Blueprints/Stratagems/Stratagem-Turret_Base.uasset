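; Base turret stratagem actor that automatically targets and fires at aliens overlapping it.
; Each tick it picks a target from overlapping Alien_Base actors, starting with the first and stopping at the first one that is as close or closer.
; It then rotates the Turret component toward that target.
; A delta-time accumulator compared to FireRate paces projectile spawns from FireDirection, each with a firing sound.
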(event `self.ReceiveTick`
  (params (DeltaSeconds :type "Float (single-precision)"))
  (`parent.ReceiveTick` DeltaSeconds)
  (`self.Find Closest Enemy`)
  (`self.Rotate Turret`)
  (`self.Shoot` DeltaSeconds))

(fn `Find Closest Enemy`
  (bind _overlappingactors (`self.GetOverlappingActors` "/Game/MyContent/Blueprints/Aliens/Alien_Base.Alien_Base_C"))
  ;[1 1 1] Gets all aliens in range, sets the first one as the closest (for now)
  (set `self.Closest Enemy` (`|GetArrayItem` _overlappingactors))
  ;[1 1 1] For Each Alien checks to see if it is closer then the current Closest Enemy.  If so, sets it to the new Closest Enemy
  (for (_array_element _array_index) _overlappingactors
    (if (!= _array_index 0)
      (if (<= (`self.GetDistanceTo` _array_element self) (`self.GetDistanceTo` (`self.Closest Enemy`) self))
        (set `self.Closest Enemy` _array_element)
        (return)))))

(fn `Rotate Turret`
  ;[1 1 1] Is Closest Enemy not null?
  (if (`KismetSystemLibrary.IsValid` (`self.Closest Enemy`))
    ;[1 1 1] Applies Rotation
    (`SceneComponent.K2_SetWorldRotation` (`self.Turret`) (`KismetMathLibrary.FindLookAtRotation` (`SceneComponent.GetForwardVector` (`self.Turret`)) (- (`self.K2_GetActorLocation` (`self.Closest Enemy`)) (`self.K2_GetActorLocation`))) false false)))

(fn `Shoot`
  (params (DeltaSeconds :type "Float (double-precision)"))
  ;[1 1 1] Is Closest Enemy not null?
  (if (`KismetSystemLibrary.IsValid` (`self.Closest Enemy`))
    ;[1 1 1] Controls the Fire Rate
    (bind _output_get (set `self.TimeSinceLastShot` (+ DeltaSeconds (`self.TimeSinceLastShot`))))
    (if (> _output_get (`self.FireRate`))
      ;[1 1 1] Spawns the Projectile
      (`|SpawnActorFromClass` (`self.Projectile`) (`SceneComponent.K2_GetComponentToWorld` (`self.Fire Direction`)) "Undefined" "OverrideRootScale" null null)
      ;[1 1 1] Resets Time Since Last Shot
      (set `self.TimeSinceLastShot` 0.0)
      ;[1 1 1] Play SFX
      (`AudioComponent.Play` (`self.FireSFX`) 0.0))))

(fn `UserConstructionScript`
  (`parent.UserConstructionScript`))