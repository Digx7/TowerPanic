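; GEL_Resource is a pickup actor that grants GEL to the player who overlaps it.
; On overlap with a Player, it calls GainGel on the TowerPanic_PlayerState with its AmountGained value.
; It then spawns a short-lived AmbientSound actor at its location to play the pickup cue, so the sound outlasts the pickup, and destroys itself.
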(event `self.ReceiveActorBeginOverlap`
  (params (OtherActor :type "Actor Object Reference"))
  ;[1 1 1] If overlaps player then give them the GEL
  (bind _asplayer (cast `/Game/MyContent/Blueprints/Player/Player` OtherActor))
  (`/Game/MyContent/Blueprints/Player/TowerPanic_PlayerState.GainGel` (cast `/Game/MyContent/Blueprints/Player/TowerPanic_PlayerState` (`Pawn.PlayerState` _asplayer) :!pure true) (`self.Amount Gained`))
  ;[1 1 1] Plays Pickup Sound
  (bind _returnvalue (`|SpawnActorFromClass` "/Script/Engine.AmbientSound" (`self.GetTransform`) "Undefined" "OverrideRootScale" null null))
  (`|ExecutionSequence`
    (:`then_0`
      (`self.SetLifeSpan` _returnvalue 10.0)
      (bind _audiocomponent (`AmbientSound.AudioComponent` _returnvalue))
      (`AudioComponent.SetSound` _audiocomponent "/Game/MyContent/Audio/SoundCues/Pickup_Cue.Pickup_Cue")
      (`AudioComponent.Play` _audiocomponent 0.0))
    (:`then_1`
      (`self.K2_DestroyActor`))))

(fn `UserConstructionScript`)