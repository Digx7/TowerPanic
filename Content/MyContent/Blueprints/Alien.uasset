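; Alien enemy character that chases the closest actor among its target classes, attacks it, and can be killed.
; A self-restarting AIMoveTo loop re-picks the target and asks the mutant AnimBP to attack on arrival.
; Anim notifies open a hit window in which Tick damages HurtBox overlaps, tracking actors already hit.
; Damage depletes Health; death plays through the AnimBP, then spawns a GEL_Resource and destroys the alien.
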(event `self.ReceiveBeginPlay`
  (bind _abp_mutant (`self.ABP Mutant`))
  ;[1 1 1] Set up
  (add `self.OnTakeAnyDamage` (delegate `OnTakeAnyDamage_Event`))
  (bind _asabp_mutant (cast `/Game/MyContent/Characters/Aliens/Animations/ABP_mutant` (`SkeletalMeshComponent.GetAnimInstance` (`self.Mesh`))))
  (set `self.ABP Mutant` _asabp_mutant)
  (`KismetSystemLibrary.Delay` 0.2)
  (`self.MoveToPlayer`)
  (add `/Game/MyContent/Characters/Aliens/Animations/ABP_mutant.Hit_Start` _abp_mutant (delegate `AnimNotify: Hit Start`))
  (add `/Game/MyContent/Characters/Aliens/Animations/ABP_mutant.Hit_Done` _abp_mutant (delegate `AnimNotify: Hit Done`)))

(event `AnimNotify: Hit Start`
  (set `self.IsAttacking` true))

(event `AnimNotify: Hit Done`
  (set `self.IsAttacking` false)
  (`KismetArrayLibrary.Array_Clear` (`self.ActorsAlreadyHit`)))

(event `OnTakeAnyDamage_Event` :!signature `self.OnTakeAnyDamage`
  (params (DamagedActor :type "Actor Object Reference") (Damage :type "Float (single-precision)") (DamageType :type "DamageType Object Reference") (InstigatedBy :type "Controller Object Reference") (DamageCauser :type "Actor Object Reference"))
  ;[1 1 1] Health
  (bind _isdead (`self.HealthManger` Damage))
  ;[1 1 1] Kill
  (bind _output_get (set `self.IsDead` _isdead))
  (if _output_get
    (`/Game/MyContent/Characters/Aliens/Animations/ABP_mutant.TryToKill` (`self.ABP Mutant`))
    (`MovementComponent.StopMovementImmediately` (`self.CharacterMovement`))
    (`self.SetActorEnableCollision` false)
    (`KismetSystemLibrary.Delay` 5.0)
    (`|SpawnActorFromClass` "/Game/MyContent/Blueprints/GEL_Resource.GEL_Resource_C" (`self.GetTransform`) "Undefined" "OverrideRootScale" null null)
    (`self.K2_DestroyActor`)))

(event `MoveToPlayer`
  ;[1 1 1] Move & Attack
  (if (not (`self.IsDead`))
    (`self.Find Closest Target`)
    (`|AIMoveTo` self (0.0 0.0 0.0) (`self.ClosestActor`) 100.0
      (:`then`
        (`KismetSystemLibrary.Delay` 3.0)
        (`self.MoveToPlayer`))
      (:`OnSuccess`
        (`/Game/MyContent/Characters/Aliens/Animations/ABP_mutant.TryToAttack` (`self.ABP Mutant`))
        (`KismetSystemLibrary.Delay` 5.0)
        (`self.MoveToPlayer`))
      (:`OnFail`
        (`KismetSystemLibrary.Delay` 0.2)
        (`self.MoveToPlayer`)))))

(event `self.ReceiveTick`
  (params (DeltaSeconds :type "Float (single-precision)"))
  (if (`self.IsAttacking`)
    (for _array_element (`PrimitiveComponent.GetOverlappingActors` (`self.Hurt Box`) null)
      (if (`KismetArrayLibrary.Array_Contains` (`self.ActorsAlreadyHit`) _array_element)
        (break)
        (else
          (`GameplayStatics.ApplyDamage` _array_element (`self.Base Damage`))
          (`KismetArrayLibrary.Array_Add` (`self.ActorsAlreadyHit`) _array_element))))))

(fn `Find Closest Target`
  (for _array_element (`self.ActorsToAttack`)
    (bind _outactors (`GameplayStatics.GetAllActorsOfClass` _array_element))
    (`/Engine/EditorBlueprintResources/StandardMacros.IsValid` (`self.ClosestActor`)
      (:`Is Valid`
        (bind (_distance _returnvalue) (`GameplayStatics.FindNearestActor` (`self.K2_GetActorLocation`) _outactors))
        (if (< _distance (`self.GetDistanceTo` (`self.ClosestActor`)))
          (set `self.ClosestActor` _returnvalue)))
      (:`Is Not Valid`
        (set `self.ClosestActor` _returnvalue))))
  (return))

(fn `HealthManger`
  (params (B :type "Float (double-precision)"))
  (returns (IsDead :type Boolean))
  (bind _output_get (set `self.Health` (- (`self.Health`) B)))
  (if (<= _output_get 0.0)
    (return true)
    (else
      (return false))))

(fn `UserConstructionScript`)