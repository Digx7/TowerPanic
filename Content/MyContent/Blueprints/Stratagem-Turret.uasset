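; Stratagem turret actor that automatically targets and fires at Alien actors overlapping it.
; Each Tick picks a target by distance from the overlapping Aliens, stopping at the first one no farther than the initial entry, so it is not always the closest.
; The turret turns toward targets within SensorRange, while projectiles spawn from FireDirection on a FireRate interval whenever a target is valid, regardless of that range.
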(event `self.ReceiveTick`
  (params (DeltaSeconds :type "Float (single-precision)"))
  (`parent.ReceiveTick` DeltaSeconds)
  (`self.Find Closest Enemy`)
  (`self.Rotate Turret`)
  (`self.Shoot` DeltaSeconds))

(fn `Find Closest Enemy`
  (bind _overlappingactors (`self.GetOverlappingActors` "/Game/MyContent/Blueprints/Alien.Alien_C"))
  (set `self.Closest Enemy` (`|GetArrayItem` _overlappingactors))
  (for (_array_element _array_index) _overlappingactors
    (if (!= _array_index 0)
      (if (<= (`self.GetDistanceTo` _array_element self) (`self.GetDistanceTo` (`self.Closest Enemy`) self))
        (set `self.Closest Enemy` _array_element)
        (return)))))

(fn `Rotate Turret`
  (bind _returnvalue (- (`self.K2_GetActorLocation` (`self.Closest Enemy`)) (`self.K2_GetActorLocation`)))
  (if (`KismetSystemLibrary.IsValid` (`self.Closest Enemy`))
    (if (< (`KismetMathLibrary.VSize` _returnvalue) (`self.Sensor Range`))
      (`SceneComponent.K2_SetWorldRotation` (`self.Turret`) (`KismetMathLibrary.FindLookAtRotation` (`SceneComponent.GetForwardVector` (`self.Turret`)) _returnvalue) false false))))

(fn `Shoot`
  (params (DeltaSeconds :type "Float (double-precision)"))
  (if (`KismetSystemLibrary.IsValid` (`self.Closest Enemy`))
    (bind _output_get (set `self.TimeSinceLastShot` (+ DeltaSeconds (`self.TimeSinceLastShot`))))
    (if (> _output_get (`self.FireRate`))
      (`|SpawnActorFromClass` (`self.Projectile`) (`SceneComponent.K2_GetComponentToWorld` (`self.Fire Direction`)) "Undefined" "OverrideRootScale" null null)
      (set `self.TimeSinceLastShot` 0.0))))

(fn `UserConstructionScript`
  (`parent.UserConstructionScript`))