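; Player state for Tower Panic that tracks the player's health and Gel, a spendable resource.
; Damage and Heal feed UpdateHealth, which adds the unclamped change and fires the IsDead dispatcher at zero or below.
; BeginPlay adds MaxHealth to current health through the same function.
; GainGel and SpendGel feed UpdateGel, with SpendGel checking affordability first and returning whether payment succeeded.
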(event `self.ReceiveBeginPlay`
  ;[1 1 1] Setup
  (`self.UpdateHealth` (`self.MaxHealth`)))

(fn `Damage`
  (params (DamageAmount :type "Float (double-precision)"))
  (`self.UpdateHealth` (* DamageAmount -1.0)))

(fn `GainGel`
  (params (AmountGained :type Integer))
  (`self.UpdateGel` AmountGained))

(fn `Heal`
  (params (HealAmount :type "Float (double-precision)"))
  (`self.UpdateHealth` HealAmount))

(fn `SpendGel`
  (params (AmountToPay :type Integer))
  (returns (CouldYouPay :type Boolean))
  ;[1 1 1] Checks if you can afford it
  (if (>= (`self.CurrentGel`) AmountToPay)
    (`self.UpdateGel` (* AmountToPay -1))
    (return true)
    (else
      (return false))))

(fn `UpdateGel`
  (params (Update :type Integer))
  (set `self.CurrentGel` (+ Update (`self.CurrentGel`))))

(fn `UpdateHealth`
  (params (Update :type "Float (double-precision)"))
  ;[1 1 1] Updates Health
  (bind _output_get (set `self.CurrentHealth` (+ Update (`self.CurrentHealth`))))
  ;[1 1 1] Checks if is dead
  (if (<= _output_get 0.0)
    (`self.IsDead` true)))

(fn `UserConstructionScript`)