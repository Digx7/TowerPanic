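; TowerPanic player state that tracks the player's health and a spendable Gel resource.
; Health starts at MaxHealth on BeginPlay, and Damage and Heal feed UpdateHealth, which calls IsDead once health reaches zero or below, with no upper clamp.
; GainGel and SpendGel adjust Gel through UpdateGel, with SpendGel returning false when the balance cannot cover the cost.
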(event `self.ReceiveBeginPlay`
  (`self.UpdateHealth` (`self.MaxHealth`)))

(fn `Damage`
  (params (DamageAmount :type "Float (double-precision)"))
  (`self.UpdateHealth` (* DamageAmount -1.0)))

(fn `GainGel`
  (params (AmountGained :type Integer))
  (`self.UpdateGel` AmountGained))

(fn `Heal`
  (params (HealAmount :type "Float (double-precision)"))
  (`self.UpdateHealth` HealAmount))

(fn `SpendGel`
  (params (AmountToPay :type Integer))
  (returns (CouldYouPay :type Boolean))
  (if (<= AmountToPay (`self.CurrentGel`))
    (`self.UpdateGel` (* AmountToPay -1))
    (return true)
    (else
      (return false))))

(fn `UpdateGel`
  (params (Update :type Integer))
  (set `self.CurrentGel` (+ Update (`self.CurrentGel`))))

(fn `UpdateHealth`
  (params (Update :type "Float (double-precision)"))
  (bind _output_get (set `self.CurrentHealth` (+ Update (`self.CurrentHealth`))))
  (if (<= _output_get 0.0)
    (`self.IsDead` true)))

(fn `UserConstructionScript`)