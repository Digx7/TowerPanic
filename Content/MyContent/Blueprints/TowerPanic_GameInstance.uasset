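; Game instance for Tower Panic that handles music and level transitions across level loads.
; SetupMusic creates two persistent 2D audio players once, and SwitchMusic crossfades between them by cycling the active index.
; It stores the current and next level, opens the next on request, and can set next to current.
; A dispatcher notifies listeners when the level is fading out.
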(event `CustomEvent_Call_LevelFadingOut_GameInstance`
  (`self.On_LevelFadingOut_GameInstance`) ; Actors in the scene can listen to this for when the level is fading out
)

(event `CustomEvent_OpenNextLevel`
  (bind _nextlevel (`self.NextLevel`))
  (`GameplayStatics.OpenLevelBySoftObjectPtr` _nextlevel)
  (set `self.CurrentLevel` _nextlevel))

(fn `Get Next Song Index`
  ;[1 1 1] Sets NextSongIndex
  (bind _output_get (set `self.Next Song Index` (+ (`self.Active Player Index`) 1)))
  ;[1 1 1] If NextSongIndex is larger than AudioPlayers length then we set it to 0
  (if (>= _output_get (`KismetArrayLibrary.Array_Length` (`self.AudioPlayers`)))
    (set `self.Next Song Index` 0)))

(fn `Play Music`
  (params (NewSong :type "SoundBase Object Reference"))
  (bind _output (`|GetArrayItem` (`self.AudioPlayers`) (`self.Active Player Index`)))
  (`AudioComponent.SetSound` _output NewSong)
  (`AudioComponent.Play` _output 0.0))

(fn `SetNextLevel`
  (params (NextLevel :type "World Soft Object Reference"))
  (set `self.NextLevel` NextLevel))

(fn `SetNextLevelToCurrentLevel`
  (set `self.NextLevel` (`self.CurrentLevel`)))

(fn `Setup Music`
  (bind _audioplayers (`self.AudioPlayers`))
  (if (not (`self.Have Songs Been Setup`))
    (bind _returnvalue (`GameplayStatics.CreateSound2D` "/Game/MyContent/Audio/SoundWaves/Two_Steps_From_Hell_-_Star_Sky__Instrumental_.Two_Steps_From_Hell_-_Star_Sky__Instrumental_" 1.0 1.0 0.0 null true false)) ; Creates a persistant audio player we can use to fade to and from for music transitions
    (`KismetArrayLibrary.Array_Add` _audioplayers _returnvalue)
    (bind _returnvalue_2 (`GameplayStatics.CreateSound2D` "/Game/MyContent/Audio/SoundWaves/Two_Steps_From_Hell_-_Battleborne__Instrumental__.Two_Steps_From_Hell_-_Battleborne__Instrumental__" 1.0 1.0 0.0 null true false)) ; Creates a persistant audio player we can use to fade to and from for music transitions
    (`KismetArrayLibrary.Array_Add` _audioplayers _returnvalue_2)
    (set `self.Have Songs Been Setup` true)))

(fn `Switch Music`
  (params (NewSong :type "SoundBase Object Reference") (Duration :type "Float (single-precision)"))
  (bind _output (`|GetArrayItem` (`self.AudioPlayers`) (`self.Next Song Index`)))
  ;[1 1 1] Sets up next song
  (`self.Get Next Song Index`)
  (`AudioComponent.SetSound` _output NewSong)
  ;[1 1 1] Fade In/Out
  (`AudioComponent.FadeIn` _output Duration 1.0 0.0 "Linear")
  (`AudioComponent.FadeOut` (`|GetArrayItem` (`self.AudioPlayers`) (`self.Active Player Index`)) Duration 0.0 "Linear")
  (set `self.Active Player Index` (`self.Next Song Index`)))