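; Wave manager for TowerPanic that schedules alien waves and detects when the player has won.
; After an initial delay, it calls NewWave, starts every alien spawner with the current wave index, then re-triggers itself on a timed delay until the wave count is reached.
; On the last wave, a delayed Tick check looks for remaining Alien actors and tells the game state the player won when none are left.
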(event `self.ReceiveBeginPlay`
  (`KismetSystemLibrary.Delay` (`self.TimeTellFirstWave`))
  (`self.Event StartNextWave`))

(event `self.ReceiveTick`
  (params (DeltaSeconds :type "Float (single-precision)"))
  (if (`self.OnLastWave`)
    (`KismetSystemLibrary.Delay` 1.0)
    (bind _returnvalue (`GameplayStatics.GetActorOfClass` "/Game/MyContent/Blueprints/Aliens/Alien.Alien_C"))
    (`/Engine/EditorBlueprintResources/StandardMacros.IsValid` _returnvalue
      (:`Is Not Valid`
        (`/Game/MyContent/Blueprints/TowerPanic_GameState.CustomEvent_PlayerWon` (cast `/Game/MyContent/Blueprints/TowerPanic_GameState` (`GameplayStatics.GetGameState`) :!pure true))))))

(event `Event StartNextWave`
  (`self.NewWave`)
  (for _array_element (`self.AlienSpawners`)
    (`/Game/MyContent/Blueprints/Aliens/Alien_Spawner.StartSpawning` _array_element (`self.CurrentWaveIndex`)))
  (bind _result (`/Engine/EditorBlueprintResources/StandardMacros.IncrementInt` (`self.CurrentWaveIndex`))
    (:`  `
      (`KismetSystemLibrary.Delay` (`self.TimeBetweenWaves`))
      (if (< _result (`self.NumberOfWaves`))
        (`self.Event StartNextWave`)
        (else
          (set `self.OnLastWave` true))))))

(fn `UserConstructionScript`)