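; Alien spawner actor that spawns random aliens at its own location for each wave.
; StartSpawning sets the current wave and enables spawning if that wave's entry in AmountToSpawn is non-zero.
; Tick accumulates time against a random delay between the min and max spawn rates, spawning a random AliensToSpawn class through SpawnAIFromClass.
; It re-rolls the delay after spawns until the wave's count is reached, then stops and resets the counter.
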(event `StartSpawning`
  (params (NewWave :type Integer))
  (bind _output_get (set `self.CurrentWave` NewWave))
  (if (!= (`|GetArrayItem` (`self.AmountToSpawn`) _output_get) 0)
    (set `self.ShouldSpawn` true)))

(event `self.ReceiveTick`
  (params (DeltaSeconds :type "Float (single-precision)"))
  (if (`self.ShouldSpawn`)
    ;[1 1 1] Spawn Trigger
    (`|ExecutionSequence`
      (:`then_0`
        (`/Engine/EditorBlueprintResources/StandardMacros.DoOnce` false
          (:`Completed`
            ;[1 1 1] Reset Spawn Trigger
            (set `self.Next Spawn Time` (`KismetMathLibrary.RandomFloatInRange` (`self.MinSpawnRate`) (`self.MaxSpawnRate`)) :!label _label))))
      (:`then_1`
        (bind _output_get (set `self.CurrentTime` (+ DeltaSeconds (`self.CurrentTime`))))
        (if (> _output_get (`self.Next Spawn Time`))
          ;[1 1 1] Where To Spawn
          (`self.SpawnAlien` (`KismetArrayLibrary.Array_Random` (`self.AliensToSpawn`)))
          (set `self.CurrentTime` 0.0)
          (bind _result (`/Engine/EditorBlueprintResources/StandardMacros.IncrementInt` (`self.AmountAlreadySpawned`))
            (:`  `
              (if (< _result (`|GetArrayItem` (`self.AmountToSpawn`) (`self.CurrentWave`)))
                (goto _label)
                (else
                  (set `self.ShouldSpawn` false)
                  (set `self.AmountAlreadySpawned` 0))))))))))

(fn `SpawnAlien`
  (params (AlienToSpawn :type "Pawn Class Reference"))
  (`AIBlueprintHelperLibrary.SpawnAIFromClass` AlienToSpawn null (`self.K2_GetActorLocation`) (struct) false null))

(fn `UserConstructionScript`)