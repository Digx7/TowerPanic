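; Alien spawner actor that periodically spawns a random AI alien at its own location.
; Tick rolls a first spawn delay once via DoOnce, then accumulates DeltaSeconds into a timer.
; When the timer exceeds the delay, it spawns a random class from AliensToSpawn, resets, and rolls a new delay between the min and max spawn rates.
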(event `self.ReceiveTick`
  (params (DeltaSeconds :type "Float (single-precision)"))
  (`|ExecutionSequence`
    (:`then_0`
      (`/Engine/EditorBlueprintResources/StandardMacros.DoOnce` false
        (:`Completed`
          (set `self.Next Spawn Time` (`KismetMathLibrary.RandomFloatInRange` (`self.MinSpawnRate`) (`self.MaxSpawnRate`)) :!label _label))))
    (:`then_1`
      (bind _output_get (set `self.CurrentTime` (+ DeltaSeconds (`self.CurrentTime`))))
      (if (> _output_get (`self.Next Spawn Time`))
        (`AIBlueprintHelperLibrary.SpawnAIFromClass` (`KismetArrayLibrary.Array_Random` (`self.AliensToSpawn`)) null (`self.K2_GetActorLocation`) (struct) false null)
        (set `self.CurrentTime` 0.0)
        (goto _label)))))

(fn `UserConstructionScript`)